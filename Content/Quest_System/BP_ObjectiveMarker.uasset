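; BP_ObjectiveMarker is a quest objective marker actor that completes the objective when touched by the player.
; Overlap of its sphere by an actor tagged Player calls CompleteObjective on the quest manager reference, then destroys the marker.
; A looping timer runs UpdateDistance, which checks the player's distance against a threshold but acts on neither result; its distance text formatting nodes are unused.
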(event `self.ReceiveBeginPlay`
  (`KismetSystemLibrary.K2_SetTimer` null "UpdateDistance" 0.2 true))

(event `self.Sphere.OnComponentBeginOverlap`
  (params (OverlappedComponent :type "PrimitiveComponent Object Reference") (OtherActor :type "Actor Object Reference") (OtherComp :type "PrimitiveComponent Object Reference") (OtherBodyIndex :type Integer) (bFromSweep :type Boolean) (SweepResult :type "HitResult Structure (by ref)"))
  (if (`self.ActorHasTag` OtherActor "Player")
    (`/Game/Quest_System/BP_QuestManager.CompleteObjective` (`self.QuestManagerRef`))
    (`self.K2_DestroyActor`)))

(fn `UpdateDistance`
  (if (< (`self.GetDistanceTo` (`GameplayStatics.GetPlayerPawn` 0)) 1000.0)
    _))

(fn `UserConstructionScript`)